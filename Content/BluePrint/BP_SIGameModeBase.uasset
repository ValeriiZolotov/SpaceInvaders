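; BP_SIGameModeBase is a game mode Blueprint that switches the on-screen UI between the HUD and the win and lose screens.
; BeginPlay calls CreatHUD to show the HUD widget, while the Win and Loose events show BP_Win and BP_Lost.
; Each of these events removes all existing widgets before creating its own and adding it to the viewport.
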(event Custom|CreatHUD
  (Viewport|RemoveAllWidgets)
  (bind _returnvalue (UserInterface|CreateWidget "/Game/BluePrint/HUD.HUD_C"))
  (UserInterface|Viewport|AddtoViewport _returnvalue 0))

(event EventBeginPlay
  (CallFunction|CreatHUD))

(event EventTick
  (params (DeltaSeconds :type Float%20%28single-precision%29)))

(event EventLoose
  (Viewport|RemoveAllWidgets)
  (bind _returnvalue (UserInterface|CreateWidget "/Game/BluePrint/BP_Lost.BP_Lost_C"))
  (UserInterface|Viewport|AddtoViewport _returnvalue 0))

(event EventWin
  (Viewport|RemoveAllWidgets)
  (bind _returnvalue (UserInterface|CreateWidget "/Game/BluePrint/BP_Win.BP_Win_C"))
  (UserInterface|Viewport|AddtoViewport _returnvalue 0))

(fn ConstructionScript)